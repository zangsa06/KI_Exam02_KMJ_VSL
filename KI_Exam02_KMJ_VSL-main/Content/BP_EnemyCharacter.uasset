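; Enemy character that chases the player, deals damage on contact and drops a coin on death.
; After a startup delay it sets health and walk speed, then loops AI MoveTo toward the player.
; Tick applies frame-time-scaled damage to every overlapping actor, while player overlap with its Box subtracts its own attack value from its health.
; At zero health it spawns BP_Coin, increments player score, ragdolls and is destroyed.
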(event `self.ReceiveBeginPlay`
  (`KismetSystemLibrary.Delay` 1.5)
  (set `self.EnemyCurrentHealth` (`self.EnemyMaxHealth`))
  (set `CharacterMovementComponent.MaxWalkSpeed` (`self.최대 걷기 속도`) (`self.CharacterMovement`))
  (`|AIMoveTo` self (0.0 0.0 0.0) (`GameplayStatics.GetPlayerCharacter` 0) :!label _label
    (:`then`
      (`KismetSystemLibrary.Delay` 0.2)
      (goto _label))))

(event `self.Box.OnComponentBeginOverlap`
  (params (OverlappedComponent :type "PrimitiveComponent Object Reference") (OtherActor :type "Actor Object Reference") (OtherComp :type "PrimitiveComponent Object Reference") (OtherBodyIndex :type Integer) (bFromSweep :type Boolean) (SweepResult :type "HitResult Structure (by ref)"))
  (cast `/Game/TopDown/Blueprints/BP_TopDownCharacter` OtherActor)
  (set `self.EnemyCurrentHealth` (- (`self.EnemyCurrentHealth`) (`self.EnemyAD`))))

(event `self.ReceiveTick`
  (params (DeltaSeconds :type "Float (single-precision)"))
  (`self.CheckEnemyLife`)
  (`self.CheckDamage`))

(event `CheckEnemyLife`
  (bind (_returnvalue_location _returnvalue_rotation) (`KismetMathLibrary.BreakTransform` (`self.GetTransform`)))
  (if (<= (`self.EnemyCurrentHealth`) 0.0)
    (`/Engine/EditorBlueprintResources/StandardMacros.DoOnce` false
      (:`Completed`
        (`|SpawnActorFromClass` "/Game/TopDown/Blueprints/BP_Coin.BP_Coin_C" (`KismetMathLibrary.MakeTransform` _returnvalue_location _returnvalue_rotation) "AdjustIfPossibleButAlwaysSpawn" "MultiplyWithRoot" null null)
        (bind _asbp_top_down_character (cast `/Game/TopDown/Blueprints/BP_TopDownCharacter` (`GameplayStatics.GetPlayerCharacter` 0)))
        (set `/Game/TopDown/Blueprints/BP_TopDownCharacter.Score` (+ (`/Game/TopDown/Blueprints/BP_TopDownCharacter.Score` _asbp_top_down_character) 1) _asbp_top_down_character)
        (`PrimitiveComponent.SetSimulatePhysics` (`self.Mesh`) true)
        (`KismetSystemLibrary.Delay` 1.0)
        (`self.K2_DestroyActor`)))))

(event `self.ReceiveActorBeginOverlap`
  (params (OtherActor :type "Actor Object Reference"))
  (`KismetArrayLibrary.Array_AddUnique` (`self.OtherActors`) OtherActor))

(event `self.ReceiveActorEndOverlap`
  (params (OtherActor :type "Actor Object Reference"))
  (`KismetArrayLibrary.Array_RemoveItem` (`self.OtherActors`) OtherActor))

(event `CheckDamage`
  (if (> (`self.EnemyCurrentHealth`) 0.0)
    (for _array_element (`self.OtherActors`)
      (`GameplayStatics.ApplyDamage` _array_element (* (`GameplayStatics.GetWorldDeltaSeconds`) (`self.EnemyAD`))))))

(fn `UserConstructionScript`)
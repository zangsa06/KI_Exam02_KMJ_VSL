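; BP_EnemySpawner is an actor that keeps spawning BP_EnemyCharacter enemies at its own transform, faster as the player levels up.
; It spawns one on BeginPlay, then Tick drives a Delay that shrinks with the BP_TopDownCharacter's Level before each further spawn.
; Each enemy spawns even when colliding, adjusting position if possible, and receives a reference back to its spawner.
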(event `self.ReceiveBeginPlay`
  (`self.SpawnEnemy` :!label _label))

(event `self.ReceiveTick`
  (params (DeltaSeconds :type "Float (single-precision)"))
  (bind _asbp_top_down_character (cast `/Game/TopDown/Blueprints/BP_TopDownCharacter` (`GameplayStatics.GetPlayerCharacter` 0)))
  (`KismetSystemLibrary.Delay` (- 7.0 (* (`/Game/TopDown/Blueprints/BP_TopDownCharacter.Level` _asbp_top_down_character) 0.5)))
  (goto _label))

(event `SpawnEnemy`
  (bind (_returnvalue_location _returnvalue_rotation) (`KismetMathLibrary.BreakTransform` (`self.GetTransform`)))
  (bind _returnvalue (`|SpawnActorFromClass` "/Game/BP_EnemyCharacter.BP_EnemyCharacter_C" (`KismetMathLibrary.MakeTransform` _returnvalue_location _returnvalue_rotation) "AdjustIfPossibleButAlwaysSpawn" "MultiplyWithRoot" null null))
  (set `/Game/BP_EnemyCharacter.Spawner` self _returnvalue))

(fn `UserConstructionScript`)
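; BP_ProjectileSpawner is an auto-aiming turret that shoots projectiles at enemy characters it sees.
; PawnSensing sightings that cast to BP_EnemyCharacter turn the Sphere toward the target using interpolated look-at pitch and yaw, with roll held at zero.
; Each sighting also restarts a short retriggerable delay, which spawns BP_Projectile at the Scene component's transform when it expires.
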(event `self.PawnSensing.OnSeePawn`
  (params (Pawn :type "Pawn Object Reference"))
  (bind _sphere (`self.Sphere`))
  (bind _asbp_enemy_character (cast `/Game/BP_EnemyCharacter` Pawn))
  (`|ExecutionSequence`
    (:`then_0`
      (bind (_returnvalue_roll _returnvalue_pitch _returnvalue_yaw) (`KismetMathLibrary.BreakRotator` (`KismetMathLibrary.RInterpTo` (`SceneComponent.RelativeRotation` _sphere) (`KismetMathLibrary.FindLookAtRotation` (`SceneComponent.K2_GetComponentLocation` _sphere) (`self.K2_GetActorLocation` _asbp_enemy_character)) (`GameplayStatics.GetWorldDeltaSeconds`) 200.0)))
      (`SceneComponent.K2_SetRelativeRotation` (`self.Sphere`) (`KismetMathLibrary.MakeRotator` 0.0 _returnvalue_pitch _returnvalue_yaw) false false))
    (:`then_1`
      (`KismetSystemLibrary.RetriggerableDelay` 0.1)
      (`|SpawnActorFromClass` "/Game/BP_Projectile.BP_Projectile_C" (`SceneComponent.K2_GetComponentToWorld` (`self.Scene`)) "Undefined" "MultiplyWithRoot" null null))))

(fn `UserConstructionScript`)